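; BP_Car is an AI-driven car pawn that parks and can later leave.
; On BeginPlay it uses AI MoveTo to reach the first BP_ParkingSpot found, marks itself parked and the spot occupied, then moves to a hard-indexed Machine actor.
; Leave moves it to BP_ExitPoint and destroys it on arrival.
; CurrentParkingSpot is never assigned here and is cleared before Leave tries to free its occupied flag.
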(event `Leave`
  (bind _returnvalue (`GameplayStatics.GetActorOfClass` "/Game/BluePrints/BP_ExitPoint.BP_ExitPoint_C"))
  (`|AIMoveTo` self (0.0 0.0 0.0) _returnvalue
    (:`OnSuccess`
      (bind _output_get (set `self.CurrentParkingSpot` null))
      (set `/Game/BluePrints/BP_ParkingSpot.IsOccupied` false _output_get)
      (`self.K2_DestroyActor`))))

(event `self.ReceiveBeginPlay`
  (bind _returnvalue (`GameplayStatics.GetActorOfClass` "/Game/BluePrints/BP_ParkingSpot.BP_ParkingSpot_C"))
  (`|AIMoveTo` self (0.0 0.0 0.0) _returnvalue
    (:`then`
      (`KismetSystemLibrary.PrintString` "IntentandoMover"))
    (:`OnSuccess`
      (set `self.IsParked` true)
      (bind _asbp_parking_spot (cast `/Game/BluePrints/BP_ParkingSpot` _returnvalue))
      (set `/Game/BluePrints/BP_ParkingSpot.IsOccupied` true _asbp_parking_spot)
      (bind _outactors (`GameplayStatics.GetAllActorsOfClass` "/Game/BluePrints/Machine.Machine_C"))
      (`|AIMoveTo` self (0.0 0.0 0.0) (`|GetArrayItem` _outactors 4)))))

(fn `UserConstructionScript`)